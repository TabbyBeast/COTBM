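; Base wolf enemy character that mirrors attack state from its AI controller and handles its own death.
; BeginPlay caches the AI_TD_Controller and creates a dynamic material instance from the mesh's first material.
; Tick copies the controller's range check into IsAttacking, debug-prints Health and calls Death whenever Health drops below one.
; Death runs an opacity timeline whose updates fade the material, stop movement, detach the controller and destroy the actor after a delay.
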(event `self.ReceiveBeginPlay`
  (bind _asai_td_controller (cast `/Game/Characters/Enemies/AI_TD_Controller` (`self.GetController`)))
  (set `self.As AI TD Controller` _asai_td_controller)
  (bind _returnvalue (`KismetMaterialLibrary.CreateDynamicMaterialInstance` (`PrimitiveComponent.GetMaterial` (`self.Mesh`) 0) "None"))
  (set `self.MI` _returnvalue))

(event `self.ReceiveTick`
  (params (DeltaSeconds :type "Float (single-precision)"))
  (bind _health (`self.Health`))
  (set `self.Is Attacking` (`/Game/Characters/Enemies/AI_TD_Controller.Attack Range Check` (`self.As AI TD Controller`)))
  (`KismetSystemLibrary.PrintString` (`KismetStringLibrary.Conv_DoubleToString` _health) true true (struct :`G` 0.66 :`B` 1.0 :`A` 1.0) 0.0)
  (if (< _health 1.0)
    (set `self.Dead` true)
    (`self.Death`)))

(event `Death`
  (bind (_direction _newtrack_0) (`Timeline|Opacity Fade` :`NewTime` 0.0)
    (:`Update`
      (`|ExecutionSequence`
        (:`then_0`
          (`KismetSystemLibrary.PrintString` (`KismetStringLibrary.Conv_DoubleToString` _newtrack_0) true true (struct :`G` 0.66 :`B` 1.0 :`A` 1.0) 0.0))
        (:`then_1`
          (`MaterialInstanceDynamic.SetScalarParameterValue` (`self.MI`) "Opacity" _newtrack_0)
          (`MovementComponent.StopMovementImmediately` (`self.CharacterMovement`))
          (`self.DetachFromControllerPendingDestroy`)
          (`KismetSystemLibrary.Delay` 3.0)
          (`self.K2_DestroyActor`))))))

(fn `UserConstructionScript`)