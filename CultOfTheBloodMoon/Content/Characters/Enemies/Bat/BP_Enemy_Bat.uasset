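; Bat enemy character that mirrors its AI controller's attack range check and handles hit reactions and death.
; HitReact plays a montage and sends the player's basic attack damage via BPI_DamageEnemy; CustomDamageEvent adds it to Health, while the death check reads HealthBat.
; Death stops movement and fades a dynamic material's opacity through a timeline.
; Movement component deactivation detaches the controller and destroys the actor after a delay.
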(event `self.ReceiveBeginPlay`
  (bind _asai_td_controller (cast `/Game/Characters/Enemies/AI_TD_Controller` (`self.GetController`)))
  (set `self.As AI TD Controller_Bat` _asai_td_controller)
  (bind _returnvalue (`KismetMaterialLibrary.CreateDynamicMaterialInstance` (`PrimitiveComponent.GetMaterial` (`self.Mesh`) 0) "None"))
  (set `self.MI_Bat` _returnvalue)
  (bind _asbp_top_down_character (cast `/Game/TopDown/Blueprints/BP_TopDownCharacter` (`GameplayStatics.GetPlayerCharacter` 0)))
  (set `self.As BP Top Down Character` _asbp_top_down_character))

(event `self.ReceiveTick`
  (params (DeltaSeconds :type "Float (single-precision)"))
  (set `self.Is Attacking_Bat` (`/Game/Characters/Enemies/AI_TD_Controller.Attack Range Check` (`self.As AI TD Controller_Bat`)))
  (`KismetSystemLibrary.PrintString` (`KismetStringLibrary.Conv_DoubleToString` (`self.Health_Bat`)) true true (struct :`G` 0.66 :`B` 1.0 :`A` 1.0) 0.0))

(event `Death`
  (`MovementComponent.StopMovementImmediately` (`self.CharacterMovement`))
  (set `self.Dead_Bat` true)
  (`|ExecutionSequence`
    (:`then_0`
      (bind (_direction _newtrack_0) (`Timeline|Opacity Fade_0`)
        (:`Update`
          (`|ExecutionSequence`
            (:`then_0`
              (`KismetSystemLibrary.PrintString` (`KismetStringLibrary.Conv_DoubleToString` _newtrack_0) true true (struct :`G` 0.66 :`B` 1.0 :`A` 1.0) 0.0))
            (:`then_1`
              (`MaterialInstanceDynamic.SetScalarParameterValue` (`self.MI_Bat`) "Opacity" _newtrack_0))))))))

(event `/Game/Characters/Enemies/BPI_DamageEnemy.Custom damage event`
  (params (DamageAmount :type "Float (double-precision)"))
  (bind _output_get (set `self.Health` (`KismetMathLibrary.FClamp` (+ (`self.Health`) DamageAmount) 0.0 100.0)))
  (`KismetSystemLibrary.PrintString` (`KismetStringLibrary.Conv_DoubleToString` _output_get))
  (`KismetSystemLibrary.RetriggerableDelay` 0.5)
  (set `self.Getting Hit Bat` false))

(event `HitReact`
  (if (not (`self.Getting Hit Bat`))
    (set `self.Getting Hit Bat` true)
    (`|PlayMontage` (`self.Mesh`) "/Game/Characters/Enemies/Bat/Bat_Hit_Montage.Bat_Hit_Montage"
      (:`then`
        (if (`KismetSystemLibrary.DoesImplementInterface` self "/Game/Characters/Enemies/BPI_DamageEnemy.BPI_DamageEnemy_C")
          (message `/Game/Characters/Enemies/BPI_DamageEnemy.Custom damage event` self (`/Game/TopDown/Blueprints/BP_TopDownCharacter.Player Basic Attack Damage` (`self.As BP Top Down Character`)))))
      (:`OnCompleted`
        (if (<= (`self.Health_Bat`) 0.0) :!label _label
          (`self.Death`)))
      (:`OnInterrupted`
        (goto _label)))))

(event `self.CharacterMovement.OnComponentDeactivated`
  (params (Component :type "ActorComponent Object Reference"))
  (`self.DetachFromControllerPendingDestroy`)
  (`KismetSystemLibrary.Delay` 3.0)
  (`self.K2_DestroyActor`))

(fn `UserConstructionScript`)