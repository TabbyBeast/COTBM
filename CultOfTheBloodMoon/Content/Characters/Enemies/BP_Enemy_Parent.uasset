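; Parent Blueprint for enemy characters, handling hit reactions, health and death.
; HitReact plays a wolf hit montage and sends itself the player's basic attack damage via BPI_DamageEnemy, with GettingHit blocking repeats until a short delay.
; Damage is added to Health; Tick and montage completion both trigger Death when it runs out.
; Death fades a dynamic material's opacity by timeline, detaches the controller, disables collision and destroys the actor after a delay.
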(event `self.ReceiveBeginPlay`
  ;[1 1 1] Begin play
  (bind _asai_td_controller (cast `/Game/Characters/Enemies/AI_TD_Controller` (`self.GetController`)))
  (set `self.As AI TD Controller` _asai_td_controller)
  (bind _returnvalue (`KismetMaterialLibrary.CreateDynamicMaterialInstance` (`PrimitiveComponent.GetMaterial` (`self.Mesh`) 0) "None"))
  (set `self.MI` _returnvalue)
  (bind _asbp_top_down_character (cast `/Game/TopDown/Blueprints/BP_TopDownCharacter` (`GameplayStatics.GetPlayerCharacter` 0)))
  (set `self.Player Ref` _asbp_top_down_character))

(event `self.ReceiveTick`
  (params (DeltaSeconds :type "Float (single-precision)"))
  (bind _health (`self.Health`))
  ;[1 1 1] Tick
  (`KismetSystemLibrary.PrintString` (`KismetStringLibrary.Conv_DoubleToString` _health) true true (struct :`G` 0.66 :`B` 1.0 :`A` 1.0) 0.0)
  (if (< _health 1.0)
    (`self.Death`)))

(event `/Game/Characters/Enemies/BPI_DamageEnemy.Custom damage event`
  (params (DamageAmount :type "Float (double-precision)"))
  ;[1 1 1] Damage
  (bind _output_get (set `self.Health` (+ (`self.Health`) DamageAmount)))
  (`KismetSystemLibrary.PrintString` (`KismetStringLibrary.Conv_DoubleToString` _output_get))
  (`KismetSystemLibrary.RetriggerableDelay` 0.3)
  (set `self.Getting Hit` false))

(event `HitReact`
  ;[1 1 1] Hit Reaction
  (if (not (`self.Getting Hit`))
    (set `self.Getting Hit` true)
    (`|PlayMontage` (`self.Mesh`) "/Game/Characters/Enemies/Wolf/Wolf_Hit_Montage.Wolf_Hit_Montage"
      (:`then`
        (if (`KismetSystemLibrary.DoesImplementInterface` self "/Game/Characters/Enemies/BPI_DamageEnemy.BPI_DamageEnemy_C")
          (message `/Game/Characters/Enemies/BPI_DamageEnemy.Custom damage event` self (`/Game/TopDown/Blueprints/BP_TopDownCharacter.Player Basic Attack Damage` (`self.Player Ref`)))))
      (:`OnCompleted`
        (if (<= (`self.Health`) 0.0) :!label _label
          (`self.Death`)))
      (:`OnInterrupted`
        (goto _label)))))

(event `Death`
  ;[1 1 1] Death
  (set `self.Dead` true)
  (`|ExecutionSequence`
    (:`then_0`
      (bind (_direction _newtrack_0) (`Timeline|Opacity Fade`)
        (:`Update`
          (`|ExecutionSequence`
            (:`then_0`
              (`KismetSystemLibrary.PrintString` (`KismetStringLibrary.Conv_DoubleToString` _newtrack_0) true true (struct :`G` 0.66 :`B` 1.0 :`A` 1.0) 0.0))
            (:`then_1`
              (`MaterialInstanceDynamic.SetScalarParameterValue` (`self.MI`) "Opacity" _newtrack_0))))))
    (:`then_1`
      (`self.DetachFromControllerPendingDestroy`)
      (`self.SetActorEnableCollision` false)
      (`KismetSystemLibrary.Delay` 3.0)
      (`self.K2_DestroyActor`))))

(fn `UserConstructionScript`)